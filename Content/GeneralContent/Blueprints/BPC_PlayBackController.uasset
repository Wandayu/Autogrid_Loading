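; Playback controller component that replays a recorded VR session on the player, driving head and hand transforms and grab states.
; A looping timer steps LoadInput through the GameRecord map in the Global_Arrays game instance, calling grab or release only on state changes.
; Playback starts paused, supports pause and resume, changes speed by rescaling the timer interval, and signals when the recording ends.
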(event Custom|BeginPlayBack
  (bind _as_global_arrays (Variables|Default|GetAs%20Global%20Arrays))
  (bind _returnvalue (Utilities|Time|SetTimerbyEvent (delegate Custom|LoadInput) (* (Variables|/Game/GeneralContent/Blueprints/Global_Arrays.Global_Arrays_C|GetRecordDeltaTime _as_global_arrays) (Variables|/Game/GeneralContent/Blueprints/Global_Arrays.Global_Arrays_C|GetSpeedFactor _as_global_arrays)) true))
  (bind _output_get (Variables|Default|SetPlayBackHandle _returnvalue))
  (Utilities|Time|PauseTimerbyHandle _output_get))

(event Custom|LoadInput
  (bind _as_global_arrays (Variables|Default|GetAs%20Global%20Arrays))
  (bind _queryindex (Variables|Default|GetqueryIndex))
  (bind _player (Variables|Default|GetPlayer))
  (bind _gamerecord (Variables|/Game/GeneralContent/Blueprints/Global_Arrays.Global_Arrays_C|GetGameRecord _as_global_arrays))
  (bind (_value _returnvalue) (Utilities|Map|Find _gamerecord _queryindex))
  (bind (_lefthandtransform _lefthandgrab _righthandtransform _righthandgrab _cameratransform) (Utilities|Struct|BreakS_InputTick _value))
  (if (<= (Variables|Default|GetqueryIndex) (Variables|/Game/GeneralContent/Blueprints/Global_Arrays.Global_Arrays_C|GetRecordTimeIndexStamp (Variables|Default|GetAs%20Global%20Arrays)))
    (if _returnvalue
      ;[0.4621 0.8388 1] Update hands state
      (Variables|Default|SetifLeftHandGrabbing _lefthandgrab)
      (Variables|Default|SetifRightHandGrabbing _righthandgrab)
      ;[0.4621 0.8388 1] Update hands and head transform
      (Transformation|SetWorldTransform (Variables|/Game/GeneralContent/Blueprints/BP_PlayBackCharacter.BP_PlayBackCharacter_C|GetCamera _player) _cameratransform false true)
      (Transformation|SetWorldTransform (Variables|/Game/VirtualRealityBP/Blueprints/BP_MotionController.BP_MotionController_C|GetMotionController (Variables|/Game/GeneralContent/Blueprints/BP_PlayBackCharacter.BP_PlayBackCharacter_C|GetLeftController _player)) _lefthandtransform false true)
      (Transformation|SetWorldTransform (Variables|/Game/VirtualRealityBP/Blueprints/BP_MotionController.BP_MotionController_C|GetMotionController (Variables|/Game/GeneralContent/Blueprints/BP_PlayBackCharacter.BP_PlayBackCharacter_C|GetRightController _player)) _righthandtransform false true)
      (CallFunction|HandleGrabbingEvent))
    ;[0.5086 1 0.5251] Update query time index
    (Math|Integer|IncrementInt (Variables|Default|GetqueryIndex))
    (else
      (Utilities|Time|ClearandInvalidateTimerbyHandle (Variables|Default|GetPlayBackHandle))
      (Default|CallPlayBackFinished))))

(event Custom|HandleGrabbingEvent
  (bind _player (Variables|Default|GetPlayer))
  (bind _player_2 (Variables|Default|GetPlayer))
  (Utilities|FlowControl|Sequence
    (:then_0
      ;[0.4621 0.8388 1] Handle left hand
      (if (Math|Boolean|NotEqual(Boolean) (Variables|Default|GetifLeftHandGrabbing) (Variables|Default|GetleftHandGrabState))
        (bind _output_get (Variables|Default|SetleftHandGrabState (Variables|Default|GetifLeftHandGrabbing)))
        (if _output_get
          (Default|GrabLeft _player)
          (else
            (Default|ReleaseLeft _player)))))
    (:then_1
      ;[0.4621 0.8388 1] Handle right hand
      (if (Math|Boolean|NotEqual(Boolean) (Variables|Default|GetifRightHandGrabbing) (Variables|Default|GetrightHandGrabState))
        (bind _output_get_2 (Variables|Default|SetrightHandGrabState (Variables|Default|GetifRightHandGrabbing)))
        (if _output_get_2
          (Default|GrabRight _player_2)
          (else
            (Default|ReleaseRight _player_2)))))))

(event Custom|ContinuePlayBack
  ;[1 1 1] Play / Pause
  (Utilities|Time|UnpauseTimerbyHandle (Variables|Default|GetPlayBackHandle)))

(event Custom|PausePlayBack
  ;[1 1 1] Play / Pause
  (Utilities|Time|PauseTimerbyHandle (Variables|Default|GetPlayBackHandle)))

(event Custom|FasterPlay
  (bind _as_global_arrays (Variables|Default|GetAs%20Global%20Arrays))
  (bind _as_global_arrays_2 (Variables|Default|GetAs%20Global%20Arrays))
  ;[1 1 1] Control play speed
  (Variables|/Game/GeneralContent/Blueprints/Global_Arrays.Global_Arrays_C|SetSpeedFactor _as_global_arrays (* (Variables|/Game/GeneralContent/Blueprints/Global_Arrays.Global_Arrays_C|GetSpeedFactor _as_global_arrays) 0.5))
  (bind _returnvalue (Utilities|Time|SetTimerbyEvent (delegate Custom|LoadInput) (* (Variables|/Game/GeneralContent/Blueprints/Global_Arrays.Global_Arrays_C|GetRecordDeltaTime _as_global_arrays_2) (Variables|/Game/GeneralContent/Blueprints/Global_Arrays.Global_Arrays_C|GetSpeedFactor _as_global_arrays_2)) true))
  (Variables|Default|SetPlayBackHandle _returnvalue))

(event Custom|SlowerPlay
  (bind _as_global_arrays (Variables|Default|GetAs%20Global%20Arrays))
  (bind _as_global_arrays_2 (Variables|Default|GetAs%20Global%20Arrays))
  ;[1 1 1] Control play speed
  (Variables|/Game/GeneralContent/Blueprints/Global_Arrays.Global_Arrays_C|SetSpeedFactor _as_global_arrays (* (Variables|/Game/GeneralContent/Blueprints/Global_Arrays.Global_Arrays_C|GetSpeedFactor _as_global_arrays) 2.0))
  (bind _returnvalue (Utilities|Time|SetTimerbyEvent (delegate Custom|LoadInput) (* (Variables|/Game/GeneralContent/Blueprints/Global_Arrays.Global_Arrays_C|GetRecordDeltaTime _as_global_arrays_2) (Variables|/Game/GeneralContent/Blueprints/Global_Arrays.Global_Arrays_C|GetSpeedFactor _as_global_arrays_2)) true))
  (Variables|Default|SetPlayBackHandle _returnvalue))

(event Custom|ReleaseBothHands
  (Default|ReleaseLeft (Variables|Default|GetPlayer))
  (Default|ReleaseRight (Variables|Default|GetPlayer)))

(event EventBeginPlay
  (bind _asglobal_arrays (Utilities|Casting|CastToGlobal_Arrays (Game|GetGameInstance)))
  (bind _output_get (Variables|Default|SetAs%20Global%20Arrays _asglobal_arrays))
  (Variables|/Game/GeneralContent/Blueprints/Global_Arrays.Global_Arrays_C|SetSpeedFactor _output_get 1.0))

(event EventTick
  (params (DeltaSeconds :type Float%20%28single-precision%29)))