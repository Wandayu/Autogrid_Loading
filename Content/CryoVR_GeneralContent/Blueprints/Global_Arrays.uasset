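; Global_Arrays holds parallel arrays that log exam steps in CryoVR.
; ExamRecordStep appends the step index, its description looked up in the IndexDescriptions map, and the current game time to three record arrays.
; It records when the log is empty or the last recorded index is nonzero, so a step 0 entry blocks further recording.
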(fn ExamRecordStep
  (params (Step :type Integer))
  (bind _stepindexrecord (Variables|Exam|GetStepIndexRecord))
  (if (>= (Utilities|Array|Length _stepindexrecord) 1)
    (if (!= 0 (Utilities|Array|Get(acopy) _stepindexrecord (- (Utilities|Array|Length _stepindexrecord) 1)))
      (Utilities|Array|Add (Variables|Exam|GetStepIndexRecord) Step :!label _label)
      (Utilities|Array|Add (Variables|Exam|GetStepDescRecord) (.Value (Utilities|Map|Find (Variables|Exam|GetIndex&%20Descriptions) Step)))
      (Utilities|Array|Add (Variables|Exam|GetStepTimeRecord) (Utilities|Time|GetTimeSeconds)))
    (else
      (goto _label))))