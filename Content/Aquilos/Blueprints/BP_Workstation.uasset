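; BP_Workstation is a workstation actor that docks the tools and cap that touch its collision zones.
; Overlaps with the screwdriver, cap pen and tweezers snap each to its named mesh socket, keeping world scale.
; The cap zone attaches the workstation cap with relative location and rotation kept.
; That same zone also hides the water surface and splash when an overlapping DewarActor is not attached.
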(event OnComponentBeginOverlap(ScrewDriver_Collision)
  (params (OverlappedComponent :type Primitive%20Component%20Object%20Reference) (OtherActor :type Actor%20Object%20Reference) (OtherComp :type Primitive%20Component%20Object%20Reference) (OtherBodyIndex :type Integer) (bFromSweep :type Boolean) (SweepResult :type Hit%20Result%20Structure%20%28by%20ref%29))
  (bind _asbp_screw_driver (Utilities|Casting|CastToBP_ScrewDriver OtherActor))
  (Transformation|AttachComponentToComponent _asbp_screw_driver (Variables|Debug|GetStaticMeshComponent) "ScrewDriverSocket" "SnapToTarget" "SnapToTarget" "KeepWorld" true))

(event OnComponentBeginOverlap(CapPen_Collision)
  (params (OverlappedComponent :type Primitive%20Component%20Object%20Reference) (OtherActor :type Actor%20Object%20Reference) (OtherComp :type Primitive%20Component%20Object%20Reference) (OtherBodyIndex :type Integer) (bFromSweep :type Boolean) (SweepResult :type Hit%20Result%20Structure%20%28by%20ref%29))
  (bind _asbp_clippen (Utilities|Casting|CastToBP_Clippen OtherActor))
  (Transformation|AttachComponentToComponent _asbp_clippen (Variables|Debug|GetStaticMeshComponent) "CapPenSocket" "SnapToTarget" "SnapToTarget" "KeepWorld" true))

(event OnComponentBeginOverlap(Tweezers_Collision)
  (params (OverlappedComponent :type Primitive%20Component%20Object%20Reference) (OtherActor :type Actor%20Object%20Reference) (OtherComp :type Primitive%20Component%20Object%20Reference) (OtherBodyIndex :type Integer) (bFromSweep :type Boolean) (SweepResult :type Hit%20Result%20Structure%20%28by%20ref%29))
  (bind _asbp_tweezers (Utilities|Casting|CastToBP_Tweezers OtherActor))
  (Transformation|AttachComponentToComponent _asbp_tweezers (Variables|Debug|GetStaticMeshComponent) "TweezersSocket" "SnapToTarget" "SnapToTarget" "KeepWorld" true))

(event OnComponentBeginOverlap(Cap_Collision)
  (params (OverlappedComponent :type Primitive%20Component%20Object%20Reference) (OtherActor :type Actor%20Object%20Reference) (OtherComp :type Primitive%20Component%20Object%20Reference) (OtherBodyIndex :type Integer) (bFromSweep :type Boolean) (SweepResult :type Hit%20Result%20Structure%20%28by%20ref%29))
  (Utilities|FlowControl|Sequence
    (:then_0
      (bind _asbp_workstation_cap (Utilities|Casting|CastToBP_Workstation_Cap OtherActor))
      (Transformation|AttachComponentToComponent _asbp_workstation_cap (Variables|Debug|GetStaticMeshComponent) "CapSocket" "KeepRelative" "KeepRelative" "KeepWorld" true))
    (:then_1
      (bind _asdewar_actor (Utilities|Casting|CastToDewarActor OtherActor))
      (if (not (Variables|/Game/Aquilos/Blueprints/DewarActor.DewarActor_C|GetIsAttached _asdewar_actor))
        (Rendering|SetVisibility (Variables|Default|GetWater_Surface) false false)
        (Rendering|SetVisibility (Variables|Default|GetWater_Splash) false false)))))

(event EventBeginPlay)

(event Collision|EventActorBeginOverlap
  (params (OtherActor :type Actor%20Object%20Reference)))

(event EventTick
  (params (DeltaSeconds :type Float%20%28single-precision%29)))

(fn ConstructionScript)