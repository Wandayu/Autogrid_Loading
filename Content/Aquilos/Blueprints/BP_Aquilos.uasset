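; BP_Aquilos is an actor with a button-area trigger box that adjusts the VR hand gesture near its buttons.
; When a motion controller's index finger collider enters the box and the hand is not grasping, it sets that controller's index-finger-only flag.
; Any overlap end from a motion controller clears the flag, without checking which component left.
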(event OnComponentBeginOverlap(Box_Button_Hand_Gesture)
  (params (OverlappedComponent :type Primitive%20Component%20Object%20Reference) (OtherActor :type Actor%20Object%20Reference) (OtherComp :type Primitive%20Component%20Object%20Reference) (OtherBodyIndex :type Integer) (bFromSweep :type Boolean) (SweepResult :type Hit%20Result%20Structure%20%28by%20ref%29))
  ;[1 1 1] Change empty hand gesture if close to buttons
  (bind _asbp_motion_controller (Utilities|Casting|CastToBP_MotionController OtherActor))
  (if (and (== (Variables|/Game/VirtualRealityBP/Blueprints/BP_MotionController.BP_MotionController_C|GetIndexFingerColli _asbp_motion_controller) OtherComp) (not (Variables|/Game/VirtualRealityBP/Blueprints/BP_MotionController.BP_MotionController_C|GetisGrasp _asbp_motion_controller)))
    (Variables|/Game/VirtualRealityBP/Blueprints/BP_MotionController.BP_MotionController_C|SetifOnlyIndexFinger _asbp_motion_controller true)))

(event OnComponentEndOverlap(Box_Button_Hand_Gesture)
  (params (OverlappedComponent :type Primitive%20Component%20Object%20Reference) (OtherActor :type Actor%20Object%20Reference) (OtherComp :type Primitive%20Component%20Object%20Reference) (OtherBodyIndex :type Integer))
  ;[1 1 1] Change empty hand gesture if close to buttons
  (bind _asbp_motion_controller (Utilities|Casting|CastToBP_MotionController OtherActor))
  (Variables|/Game/VirtualRealityBP/Blueprints/BP_MotionController.BP_MotionController_C|SetifOnlyIndexFinger _asbp_motion_controller false))

(event EventBeginPlay)

(event Collision|EventActorBeginOverlap
  (params (OtherActor :type Actor%20Object%20Reference)))

(event EventTick
  (params (DeltaSeconds :type Float%20%28single-precision%29)))

(fn ConstructionScript)