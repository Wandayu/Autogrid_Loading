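; DewarActor is a VR-interactable dewar that accepts a cap and can be grasped by a motion controller.
; A cap entering the cap box snaps to CapSocket and switches off the frozen effect, which returns when the cap leaves.
; A motion controller touching the hand capsule triggers a hand-animation update with a defined pick on the dewar socket.
; Tick contains only empty grasp and step-recording checks.
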(event OnComponentBeginOverlap(BoxCompCap)
  (params (OverlappedComponent :type Primitive%20Component%20Object%20Reference) (OtherActor :type Actor%20Object%20Reference) (OtherComp :type Primitive%20Component%20Object%20Reference) (OtherBodyIndex :type Integer) (bFromSweep :type Boolean) (SweepResult :type Hit%20Result%20Structure%20%28by%20ref%29))
  (bind _asdewar_cap_actor (Utilities|Casting|CastToDewarCapActor OtherActor))
  (Variables|Default|SetIsAttached true)
  (Transformation|AttachComponentToComponent _asdewar_cap_actor (Variables|Default|GetStaticMeshComponent) "CapSocket" "SnapToTarget" "SnapToTarget" "KeepWorld" true)
  (Components|Activation|SetActive (Variables|Default|GetFrozenFX) false false))

(event OnComponentEndOverlap(BoxCompCap)
  (params (OverlappedComponent :type Primitive%20Component%20Object%20Reference) (OtherActor :type Actor%20Object%20Reference) (OtherComp :type Primitive%20Component%20Object%20Reference) (OtherBodyIndex :type Integer))
  (Utilities|Casting|CastToDewarCapActor OtherActor)
  (Variables|Default|SetIsAttached false)
  (Components|Activation|SetActive (Variables|Default|GetFrozenFX) true false))

(event OnComponentBeginOverlap(HandCapsuleComp)
  (params (OverlappedComponent :type Primitive%20Component%20Object%20Reference) (OtherActor :type Actor%20Object%20Reference) (OtherComp :type Primitive%20Component%20Object%20Reference) (OtherBodyIndex :type Integer) (bFromSweep :type Boolean) (SweepResult :type Hit%20Result%20Structure%20%28by%20ref%29))
  (bind _asbp_motion_controller (Utilities|Casting|CastToBP_MotionController OtherActor))
  (CallFunction|UpdateHandAniFunc _asbp_motion_controller 1.82 1.0 "Dewar_Socket" "SnapToTarget" "1.000000,1.000000,1.000000" true))

(event EventBeginPlay
  (|CallParentFunction)
  (bind _asglobal_arrays (Utilities|Casting|CastToGlobal_Arrays (Game|GetGameInstance)))
  (Variables|Default|SetGA _asglobal_arrays))

(event Collision|EventActorBeginOverlap
  (params (OtherActor :type Actor%20Object%20Reference))
  (|CallParentFunction OtherActor) ; This node is disabled and will not be called.\nDrag off pins to build functionality.
)

(event EventTick
  (params (DeltaSeconds :type Float%20%28single-precision%29))
  (|CallParentFunction DeltaSeconds)
  (if (Variables|Default|GetisGrasp)
    (if (Variables|Default|GetIsstep3Recorded)
      _)))

(fn ConstructionScript
  (|CallParentFunction))