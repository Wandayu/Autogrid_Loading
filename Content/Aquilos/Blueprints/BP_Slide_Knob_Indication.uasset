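; BP_Slide_Knob_Indication is a hand-grabbed knob that slides along a straight track between two end positions.
; Pickup stores the hand component and Drop clears it.
; While RodBottomKnob's lock status allows it, Tick projects the hand onto the segment between the first two spline points and teleports KnobBottom there.
; Tick also flips SliderPosition between Start and End when the knob comes within a small tolerance of the opposite endpoint.
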(event EventBeginPlay)

(event Collision|EventActorBeginOverlap
  (params (OtherActor :type Actor%20Object%20Reference)))

(event EventTick
  (params (DeltaSeconds :type Float%20%28single-precision%29))
  (bind _spline (Variables|Default|GetSpline))
  (Utilities|FlowControl|Sequence
    (:then_0
      ;[1 1 1] Update slider location according to hand position
      (if (Utilities|Enum|Equal(Enum) (Variables|/Game/Aquilos/Blueprints/BP_Bottom_Knob.BP_Bottom_Knob_C|GetlockStatus (Variables|Knob|GetRodBottomKnob)) "NewEnumerator1")
        (bind _hand (Variables|Default|GetHand)
          (:then
            (Transformation|SetWorldLocation (Variables|Default|GetKnob_Bottom) (Math|Vector|FindClosestPointonSegment (Transformation|GetWorldLocation _hand) (Spline|GetLocationatSplinePoint _spline 0 "World") (Spline|GetLocationatSplinePoint _spline 1 "World")) false true))
          (:else))))
    (:then_1
      ;[1 1 1] Check slider status
      (switch Utilities|FlowControl|Switch|SwitchonEnum_Slider_Position (Variables|Default|GetsliderPosition)
        (:NewEnumerator0
          (if (Math|Vector|Equal(Vector) (Transformation|GetWorldLocation (Variables|Default|GetKnob_Bottom)) (Spline|GetLocationatSplinePoint (Variables|Default|GetSpline) 1 "World") 3.0)
            (Variables|Default|SetsliderPosition "NewEnumerator1")))
        (:NewEnumerator1
          (if (Math|Vector|Equal(Vector) (Transformation|GetWorldLocation (Variables|Default|GetKnob_Bottom)) (Spline|GetLocationatSplinePoint (Variables|Default|GetSpline) 0 "World") 3.0)
            (Variables|Default|SetsliderPosition "NewEnumerator0")))))))

(event EventPickup
  (params (AttachTo :type Scene%20Component%20Object%20Reference))
  (Variables|Default|SetHand AttachTo))

(event EventDrop
  (Utilities|IsValid (Variables|Default|GetHand)
    (:Is%20Valid
      (Variables|Default|SetHand 0))))

(fn ConstructionScript)