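; Side knob actor for a rod that works as a two-position slider along a spline.
; A custom event compares the Knob's world location to the opposite spline point within a small tolerance and flips SliderPosition between Start and End on arrival.
; The graph only tracks state: it contains no movement logic, Tick just calls the parent, and nothing here calls the custom event.
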(event Custom|CustomEvent
  ;[0.5137 1 0.4118] Check slider status
  (switch Utilities|FlowControl|Switch|SwitchonEnum_Slider_Position (Variables|Default|GetsliderPosition)
    (:NewEnumerator0
      (if (Math|Vector|Equal(Vector) (Transformation|GetWorldLocation (Variables|Default|GetKnob)) (Spline|GetLocationatSplinePoint (Variables|Default|GetSpline) 1 "World") 0.5)
        (Variables|Default|SetsliderPosition "NewEnumerator1")))
    (:NewEnumerator1
      (if (Math|Vector|Equal(Vector) (Transformation|GetWorldLocation (Variables|Default|GetKnob)) (Spline|GetLocationatSplinePoint (Variables|Default|GetSpline) 0 "World") 0.5)
        (Variables|Default|SetsliderPosition "NewEnumerator0")))))

(event EventBeginPlay
  (|CallParentFunction) ; This node is disabled and will not be called.\nDrag off pins to build functionality.
)

(event Collision|EventActorBeginOverlap
  (params (OtherActor :type Actor%20Object%20Reference))
  (|CallParentFunction OtherActor) ; This node is disabled and will not be called.\nDrag off pins to build functionality.
)

(event EventTick
  (params (DeltaSeconds :type Float%20%28single-precision%29))
  (|CallParentFunction DeltaSeconds))

(fn ConstructionScript
  (|CallParentFunction))